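; BP_YSortSprite is a sprite object, named for Y-sorting, that lets its opacity be changed at runtime.
; On BeginPlay it runs the parent logic, caches the sprite's default color and binds to the OnOpacityChanged event.
; Each opacity change keeps the default RGB and multiplies the default alpha by the new value, so opacity scales relative to the original color.
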(event `self.ReceiveBeginPlay`
  (`parent.ReceiveBeginPlay`)
  (`|ExecutionSequence`
    (:`then_0`
      ;[1 1 1] Set Default Sprite Color
      (set `self.Default Color` (`PaperSpriteComponent.SpriteColor` (`self.Sprite`))))
    (:`then_1`
      ;[1 1 1] Change Sprite Opacity
      (add `self.On Opacity Changed` (delegate `ChangeSpriteOpacity`)))))

(event `ChangeSpriteOpacity` :!signature `self.On Opacity Changed`
  (params (Opacity :type "Float (double-precision)"))
  (bind (_default_color_r _default_color_g _default_color_b _default_color_a) (break `LinearColor` (`self.Default Color`)))
  ;[1 1 1] Change Sprite Opacity
  (`PaperSpriteComponent.SetSpriteColor` (`self.Sprite`) (make `LinearColor` _default_color_r _default_color_g _default_color_b (* Opacity _default_color_a))))

(fn `UserConstructionScript`
  (`parent.UserConstructionScript`))