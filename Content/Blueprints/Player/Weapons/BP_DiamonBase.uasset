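; Base actor for a diamond player weapon, built from a rotating scene, a sprite and a point light.
; Each tick it yaws DiamondScene at RotationSpeed, then counter-rotates DiamondSprite by that yaw so the sprite keeps its default orientation while the scene spins.
; On BeginPlay it tints the point light with the sprite's color.
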(event `RotateAroundCenter`
  (params (DeltaTime :type "Float (double-precision)"))
  (bind _diamondscene (`self.DiamondScene`))
  (bind (_returnvalue_roll _returnvalue_pitch _returnvalue_yaw) (`KismetMathLibrary.BreakRotator` (`SceneComponent.K2_GetComponentRotation` _diamondscene)))
  ;[1 1 1] Rotate The Actor around it's center
  (`SceneComponent.K2_SetWorldRotation` _diamondscene (`KismetMathLibrary.MakeRotator` 0.0 0.0 (+ _returnvalue_yaw (* (`self.Rotation Speed`) DeltaTime))) false false))

(event `self.ReceiveTick`
  (params (DeltaSeconds :type "Float (single-precision)"))
  (`|ExecutionSequence`
    (:`then_0`
      (`self.RotateAroundCenter` DeltaSeconds)
      (`self.RotateInnerSprite`))))

(event `RotateInnerSprite`
  (bind (_returnvalue_roll _returnvalue_pitch _returnvalue_yaw) (`KismetMathLibrary.BreakRotator` (`SceneComponent.K2_GetComponentRotation` (`self.DiamondScene`))))
  ;[1 1 1] Rotate Inner Sprite so it will be always as default rotation
  (`SceneComponent.K2_SetRelativeRotation` (`self.DiamondSprite`) (`KismetMathLibrary.MakeRotator` -90.0 0.0 (- 360.0 _returnvalue_yaw)) false false))

(event `self.ReceiveBeginPlay`
  (`|ExecutionSequence`
    (:`then_0`
      ;[1 1 1] Set Light Color based on Sprite Color
      (`LightComponent.SetLightColor` (`self.PointLight`) (`PaperSpriteComponent.SpriteColor` (`self.DiamondSprite`)) true))))

(fn `UserConstructionScript`)