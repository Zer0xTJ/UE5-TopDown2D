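; Player pawn with both direct input movement and right-click-to-move, using Enhanced Input and a visible mouse cursor.
; Right-click traces from the cursor into the world, starts a simple move to the hit point, and spawns a destination indicator there.
; Both modes set a 2D Directionality vector: raw input for direct movement, the unnormalized offset to the destination (Y flipped to match input) for clicks.
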(event `UpdateDirectionality`
  (bind (_destinationlocation_x _destinationlocation_y) (`KismetMathLibrary.BreakVector2D` (`self.destinationLocation`)))
  (bind (_returnvalue_x _returnvalue_y) (`KismetMathLibrary.BreakVector` (`SceneComponent.K2_GetComponentLocation` (`self.CapsuleComponent`))))
  (bind (_returnvalue_x_2 _returnvalue_y_2) (`KismetMathLibrary.BreakVector` (- (`KismetMathLibrary.MakeVector` _destinationlocation_x _returnvalue_y) (`KismetMathLibrary.MakeVector` _returnvalue_x _destinationlocation_y))))
  ;[1 1 1] Update Player Directionality Based on Destination
  (set `self.Directionality` (`KismetMathLibrary.MakeVector2D` _returnvalue_x_2 _returnvalue_y_2)))

(event `EnhancedInput|/Game/Inputs/Player/IA_RighMouseButtonClicked`
  (params (ActionValue :type Boolean) (ElapsedSeconds :type "Float (double-precision)") (TriggeredSeconds :type "Float (double-precision)") (InputAction :type "InputAction Object Reference" :default "/Game/Inputs/Player/IA_RighMouseButtonClicked.IA_RighMouseButtonClicked"))
  (bind (_worldlocation _worlddirection) (`PlayerController.DeprojectMousePositionToWorld` (`GameplayStatics.GetPlayerController` 0)))
  (bind (_returnvalue_x _returnvalue_y _returnvalue_z) (`KismetMathLibrary.BreakVector` (`SceneComponent.K2_GetComponentLocation` (`self.CapsuleComponent`))))
  ;[1 1 1] Move Player Using Right Click  Mouse Button
  (:`Triggered`
    (bind (_outhit _returnvalue) (`KismetSystemLibrary.LineTraceSingle` :`Start` _worldlocation :`End` (+ _worldlocation (* _worlddirection 9999999.0)) :`TraceChannel` "TraceTypeQuery1" :`DrawTime` 1.0))
    (if _returnvalue
      (bind (_bblockinghit _binitialoverlap _time _distance _location) (`GameplayStatics.BreakHitResult` _outhit))
      (set `self.destinationLocation` (`KismetMathLibrary.MakeVector2D` (.x _location) (.y _location)))
      (`AIBlueprintHelperLibrary.SimpleMoveToLocation` (`GameplayStatics.GetPlayerController` 0) (`KismetMathLibrary.MakeVector` (.x _location) (.y _location) _returnvalue_z))
      (`self.UpdateDirectionality`)
      (`|SpawnActorFromClass` "/Game/Blueprints/Indicators/BP_DestinationIndicator.BP_DestinationIndicator_C" (`KismetMathLibrary.MakeTransform` (`KismetMathLibrary.MakeVector` (.x _location) (.y _location) -20.0)) "Undefined" "MultiplyWithRoot" null null))))

(event `EnhancedInput|/Game/Inputs/Player/IA_Move`
  (params (ActionValue :type "Vector2D Structure") (ElapsedSeconds :type "Float (double-precision)") (TriggeredSeconds :type "Float (double-precision)") (InputAction :type "InputAction Object Reference" :default "/Game/Inputs/Player/IA_Move.IA_Move"))
  ;[1 1 1] Movement
  (:`Triggered`
    (`self.AddMovementInput` (1.0 0.0 0.0) ActionValue_X)
    (`self.AddMovementInput` (0.0 -1.0 0.0) ActionValue_Y)
    (set `self.Directionality` (`KismetMathLibrary.MakeVector2D` ActionValue_X ActionValue_Y))))

(event `self.ReceiveBeginPlay`
  (bind _returnvalue (pcsubsystem `EnhancedInputLocalPlayerSubsystem` (`GameplayStatics.GetPlayerController` 0)))
  (`|ExecutionSequence`
    (:`then_0`
      ;[1 1 1] Enhance Inputs
      (`/Engine/EditorBlueprintResources/StandardMacros.IsValid` _returnvalue
        (:`Is Valid`
          (`EnhancedInputSubsystemInterface.AddMappingContext` _returnvalue "/Game/Inputs/Player/IMC_Player.IMC_Player" 0 (struct)))))
    (:`then_1`
      ;[1 1 1] Show Mouse
      (set `PlayerController.bShowMouseCursor` true (`GameplayStatics.GetPlayerController` 0)))))

(fn `UserConstructionScript`)